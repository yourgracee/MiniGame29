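; Gas tank monster Blueprint that explodes into several common fire monsters some time after it first starts running.
; Tick records the time and location of the first Runing state, then destroys the tank once Boomtime elapses or horizontal travel exceeds Boomdistance.
; The blast spawns Numsplit fires at random X/Z offsets, each with a default controller.
; A widget bar shows the larger fuse progress, using signed rather than absolute X travel.
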(event `self.ReceiveTick`
  (params (DeltaSeconds :type "Float (single-precision)"))
  (`parent.ReceiveTick` DeltaSeconds)
  (`self.GetFirstTimeRun`)
  (`self.HandleBoom`)
  (`self.HandleBoomWidget`))

(event `self.ChangeSprite`
  (`self.ChangeSprite_Gas`))

(fn `ChangeSprite_Gas`
  (switch `/Game/demo/blueprint/EnumState` (`self.state`)
    (:`NewEnumerator0`
      (`PaperFlipbookComponent.SetFlipbook` (`self.Sprite`) "/Game/demo/sprites/monster/meiqi/煤气罐1.煤气罐1"))
    (:`NewEnumerator1`
      (`PaperFlipbookComponent.SetFlipbook` (`self.Sprite`) (select `bool` (`self.bisMovingRight`) :`false` "/Game/demo/sprites/monster/meiqi/煤气罐1.煤气罐1" :`true` "/Game/demo/sprites/monster/meiqi/煤气罐1.煤气罐1" :!type "PaperFlipbook Object Reference")))
    (:`NewEnumerator2`
      (`PaperFlipbookComponent.SetFlipbook` (`self.Sprite`) "/Game/demo/sprites/monster/fire/jumping.jumping"))
    (:`NewEnumerator5`
      (`PaperFlipbookComponent.SetFlipbook` (`self.Sprite`) "/Game/demo/sprites/monster/fire/dead.dead"))
    (:`NewEnumerator6`
      (`PaperFlipbookComponent.SetFlipbook` (`self.Sprite`) (select `bool` (`self.bisMovingRight`) :`false` "/Game/demo/sprites/monster/meiqi/煤气罐1.煤气罐1" :`true` "/Game/demo/sprites/monster/meiqi/煤气罐1.煤气罐1" :!type "PaperFlipbook Object Reference")))
    (:`NewEnumerator7`
      (`PaperFlipbookComponent.SetFlipbook` (`self.Sprite`) "/Game/demo/sprites/monster/meiqi/煤气罐1.煤气罐1"))))

(fn `GetFirstTimeRun`
  (if (`self.firstrun`)
    _
    (elif (`|EnumEquality` (`self.state`) "NewEnumerator1")
      (set `self.firstruntime` (`GameplayStatics.GetTimeSeconds`))
      (set `self.firstlocation` (`self.K2_GetActorLocation`))
      (set `self.firstrun` true))))

(fn `HandleBoom`
  (if (`self.firstrun`)
    (if (>= (- (`GameplayStatics.GetTimeSeconds`) (`self.firstruntime`)) (`self.boomtime`))
      (`self.K2_DestroyActor` :!label _label)
      (set `self.bDead` true)
      (`self.SpawnCommonFire`)
      (elif (> (`KismetMathLibrary.Abs` (- (.x (`self.K2_GetActorLocation`)) (.x (`self.firstlocation`)))) (`self.boomdistance`))
        (goto _label)))))

(fn `HandleBoomWidget`
  (if (`self.bDead`)
    _
    (elif (`self.firstrun`)
      (bind _asmonster_boom (cast `/Game/demo/blueprint/MonsterBoom` (`WidgetComponent.GetUserWidgetObject` (`self.BoomWidget`))))
      (`ProgressBar.SetPercent` (`/Game/demo/blueprint/MonsterBoom.MonsterBoomBar` _asmonster_boom) (`KismetMathLibrary.FMax` (/ (- (`GameplayStatics.GetTimeSeconds`) (`self.firstruntime`)) (`self.boomtime`)) (/ (- (.x (`self.K2_GetActorLocation`)) (.x (`self.firstlocation`))) (`self.boomdistance`)))))))

(fn `SpawnCommonFire`
  (for _ (range (`self.numsplit`))
    (bind _returnvalue (`|SpawnActorFromClass` "/Game/demo/blueprint/MonsterBase_CommonFire.MonsterBase_CommonFire_C" (`KismetMathLibrary.Conv_VectorToTransform` (+ (`self.K2_GetActorLocation`) (`KismetMathLibrary.MakeVector` (- (* (`KismetMathLibrary.RandomFloat`) 400.0) 50.0) 0.0 (* (`KismetMathLibrary.RandomFloat`) 200.0)))) "AdjustIfPossibleButDontSpawnIfColliding" "OverrideRootScale" null null))
    (`self.SpawnDefaultController` _returnvalue)
    (`self.init` _returnvalue)))

(fn `UserConstructionScript`
  (`parent.UserConstructionScript`))