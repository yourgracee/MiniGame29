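; Wizard boss monster for a 2D flipbook-based game that periodically summons MonsterBase_CommonFire monsters.
; Tick compares game time to the next skill time, then runs ReleaseSkill and restarts the cooldown.
; ReleaseSkill spawns several fire monsters at random X/Z offsets from the wizard, gives each a default controller, initializes it and sets it throwing.
; ChangeSprite switches on state, but every listed state uses the same boss flipbook.
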(event `self.ReceiveTick`
  (params (DeltaSeconds :type "Float (single-precision)"))
  (`parent.ReceiveTick` DeltaSeconds)
  (bind _isrelease (`self.isReleaseSkill`))
  (if _isrelease
    (`self.ReleaseSkill`)
    (`self.ResetCD`)))

(event `self.ChangeSprite`
  (`self.BossSprite`))

(fn `BossSprite`
  (switch `/Game/demo/blueprint/EnumState` (`self.state`)
    (:`NewEnumerator0`
      (`PaperFlipbookComponent.SetFlipbook` (`self.Sprite`) "/Game/demo/sprites/monster/bosssprite.bosssprite"))
    (:`NewEnumerator1`
      (`PaperFlipbookComponent.SetFlipbook` (`self.Sprite`) (select `bool` (`self.bisMovingRight`) :`false` "/Game/demo/sprites/monster/bosssprite.bosssprite" :`true` "/Game/demo/sprites/monster/bosssprite.bosssprite" :!type "PaperFlipbook Object Reference")))
    (:`NewEnumerator2`
      (`PaperFlipbookComponent.SetFlipbook` (`self.Sprite`) "/Game/demo/sprites/monster/bosssprite.bosssprite"))
    (:`NewEnumerator5`
      (`PaperFlipbookComponent.SetFlipbook` (`self.Sprite`) "/Game/demo/sprites/monster/bosssprite.bosssprite"))
    (:`NewEnumerator6`
      (`PaperFlipbookComponent.SetFlipbook` (`self.Sprite`) (select `bool` (`self.bisMovingRight`) :`false` "/Game/demo/sprites/monster/bosssprite.bosssprite" :`true` "/Game/demo/sprites/monster/bosssprite.bosssprite" :!type "PaperFlipbook Object Reference")))
    (:`NewEnumerator7`
      (`PaperFlipbookComponent.SetFlipbook` (`self.Sprite`) "/Game/demo/sprites/monster/bosssprite.bosssprite"))))

(fn `isReleaseSkill`
  (returns (isrelease :type Boolean))
  (bind _returnvalue (>= (`GameplayStatics.GetTimeSeconds`) (`self.nextskilltime`)))
  (if _returnvalue
    _
    (else
      _))
  (return _returnvalue))

(fn `ReleaseSkill`
  (for _ (range 4)
    (bind _returnvalue (`|SpawnActorFromClass` "/Game/demo/blueprint/MonsterBase_CommonFire.MonsterBase_CommonFire_C" (`KismetMathLibrary.Conv_VectorToTransform` (+ (`self.K2_GetActorLocation`) (`KismetMathLibrary.MakeVector` (- (* (`KismetMathLibrary.RandomFloat`) 400.0) 50.0) 0.0 (* (`KismetMathLibrary.RandomFloat`) 200.0)))) "AlwaysSpawn" "OverrideRootScale" null null))
    (`self.SpawnDefaultController` _returnvalue)
    (`self.init` _returnvalue)
    (`self.SetThrowing` _returnvalue)))

(fn `ResetCD`
  (set `self.nextskilltime` (+ (`GameplayStatics.GetTimeSeconds`) (`self.skillCD`))))

(fn `UserConstructionScript`
  (`parent.UserConstructionScript`))