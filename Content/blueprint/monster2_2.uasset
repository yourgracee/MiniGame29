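; A 2D monster character with a gas-canister flipbook that moves along the X axis and splits into two Monster2 actors.
; BeginPlay adds a health bar widget, starts a looping named-function timer, then after a delay destroys itself and spawns the pair with zero damage.
; Tick picks the flipbook from State, faces the controller by X velocity, and applies movement by Direction.
; Helper functions reverse Direction and remove the capsule and sprite.
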(event `self.ReceiveBeginPlay`
  ;[1 1 1] Handle Animation
  (`|ExecutionSequence`
    (:`then_0`
      (bind _returnvalue (`|CreateWidget` "/Game/demo/blueprint/zkxWidgetBlueprint.zkxWidgetBlueprint_C" (`GameplayStatics.GetPlayerController` 0)))
      (bind _output_get (set `self.healthbar` _returnvalue))
      (`UserWidget.AddToViewport` _output_get 0))
    (:`then_2`
      (`KismetSystemLibrary.K2_SetTimer` null (`self.functionstr`) 2.0 true))
    (:`then_3`
      (`KismetSystemLibrary.Delay` 5.0)
      (`self.K2_DestroyActor`)
      (bind _returnvalue_2 (`|SpawnActorFromClass` "/Game/demo/blueprint/monster2.monster2_C" (`self.GetTransform`) "AlwaysSpawn" "OverrideRootScale" null null))
      (`self.SpawnDefaultController` _returnvalue_2)
      (set `/Game/demo/blueprint/monster2.damage` 0.0 _returnvalue_2)
      (bind _returnvalue_3 (`|SpawnActorFromClass` "/Game/demo/blueprint/monster2.monster2_C" (`KismetMathLibrary.Conv_VectorToTransform` (+ (`self.K2_GetActorLocation`) (300.0 0.0 0.0))) "AlwaysSpawn" "OverrideRootScale" null null))
      (`self.SpawnDefaultController` _returnvalue_3)
      (set `/Game/demo/blueprint/monster2.damage` 0.0 _returnvalue_3))))

(event `UpdateAnimation`
  ;[1 1 1] Handle Animation
  (switch `/Game/demo/blueprint/EnumState` (`self.state`)
    (:`NewEnumerator0`
      (`PaperFlipbookComponent.SetFlipbook` (`self.Sprite`) (select `bool` (> (`KismetMathLibrary.VSize` (`self.GetVelocity`)) 0.0) :`false` "/Game/demo/sprites/monster/meiqi/煤气罐1.煤气罐1" :`true` "/Game/demo/sprites/monster/meiqi/煤气罐1.煤气罐1" :!type "PaperFlipbook Object Reference")))
    (:`NewEnumerator2`
      (`PaperFlipbookComponent.SetFlipbook` (`self.Sprite`) "/Game/demo/sprites/Jump.Jump"))
    (:`NewEnumerator5`
      (`PaperFlipbookComponent.SetFlipbook` (`self.Sprite`) "/Game/demo/sprites/dead.dead"))))

(event `self.ReceiveTick`
  (params (DeltaSeconds :type "Float (single-precision)"))
  ;[1 1 1] Tick - Updates animation
  (`|ExecutionSequence`
    (:`then_0`
      (`self.UpdateAnimation`)
      (`/Engine/EditorBlueprintResources/StandardMacros.CompareFloat` (.x (`MovementComponent.Velocity` (`self.GetMovementComponent`)))
        (:`>`
          (`Controller.SetControlRotation` (`self.GetController`) (`KismetMathLibrary.MakeRotator` 0.0) :!label _label))
        (:`==`
          (if (`self.bisMovingRight`)
            (goto _label)
            (else
              (`Controller.SetControlRotation` (`self.GetController`) (`KismetMathLibrary.MakeRotator` 0.0 0.0 180.0) :!label _label_2))))
        (:`<`
          (goto _label_2))))
    (:`then_1`
      (`self.AddMovementInput` (1.0 0.0 0.0) (`self.direction`)))))

(fn `changedirection`
  (set `self.direction` (* (`self.direction`) -1.0)))

(fn `destroycur`
  (`ActorComponent.K2_DestroyComponent` (`self.CapsuleComponent`))
  (`ActorComponent.K2_DestroyComponent` (`self.Sprite`)))

(fn `UserConstructionScript`)