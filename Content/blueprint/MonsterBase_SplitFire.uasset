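; MonsterBase_SplitFire is a flipbook-based fire monster that splits into MonsterBase_JumpFire monsters when it dies.
; Tick watches Dead, calls DestroyActor, then BeginSplit spawns Numsplit children at random X/Z offsets, skewed toward +X, each given a default controller and Init.
; SplitChangeSprites sets the same flame flipbook for every state, but nothing here calls it and the ChangeSprite event is empty.
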(event `self.ReceiveTick`
  (params (DeltaSeconds :type "Float (single-precision)"))
  (`parent.ReceiveTick` DeltaSeconds)
  (if (`self.dead`)
    (`self.K2_DestroyActor`)
    (`self.BeginSplit`)))

(event `self.ChangeSprite`)

(fn `BeginSplit`
  (for _ (range (`self.numsplit`))
    (bind _returnvalue (`|SpawnActorFromClass` "/Game/demo/blueprint/MonsterBase_JumpFire.MonsterBase_JumpFire_C" (`KismetMathLibrary.Conv_VectorToTransform` (+ (`self.K2_GetActorLocation`) (`KismetMathLibrary.MakeVector` (- (* (`KismetMathLibrary.RandomFloat`) 400.0) 50.0) 0.0 (* (`KismetMathLibrary.RandomFloat`) 200.0)))) "AdjustIfPossibleButDontSpawnIfColliding" "OverrideRootScale" null null))
    (`self.SpawnDefaultController` _returnvalue)
    (`self.init` _returnvalue)))

(fn `SplitChangeSprites`
  (switch `/Game/demo/blueprint/EnumState` (`self.state`)
    (:`NewEnumerator0`
      (`PaperFlipbookComponent.SetFlipbook` (`self.Sprite`) "/Game/demo/sprites/monster/fire/火焰3.火焰3"))
    (:`NewEnumerator1`
      (`PaperFlipbookComponent.SetFlipbook` (`self.Sprite`) (select `bool` (`self.bisMovingRight`) :`false` "/Game/demo/sprites/monster/fire/火焰3.火焰3" :`true` "/Game/demo/sprites/monster/fire/火焰3.火焰3" :!type "PaperFlipbook Object Reference")))
    (:`NewEnumerator2`
      (`PaperFlipbookComponent.SetFlipbook` (`self.Sprite`) "/Game/demo/sprites/monster/fire/火焰3.火焰3"))
    (:`NewEnumerator5`
      (`PaperFlipbookComponent.SetFlipbook` (`self.Sprite`) "/Game/demo/sprites/monster/fire/火焰3.火焰3"))
    (:`NewEnumerator6`
      (`PaperFlipbookComponent.SetFlipbook` (`self.Sprite`) (select `bool` (`self.bisMovingRight`) :`false` "/Game/demo/sprites/monster/fire/火焰3.火焰3" :`true` "/Game/demo/sprites/monster/fire/火焰3.火焰3" :!type "PaperFlipbook Object Reference")))
    (:`NewEnumerator7`
      (`PaperFlipbookComponent.SetFlipbook` (`self.Sprite`) "/Game/demo/sprites/monster/fire/火焰3.火焰3"))))

(fn `UserConstructionScript`
  (`parent.UserConstructionScript`))