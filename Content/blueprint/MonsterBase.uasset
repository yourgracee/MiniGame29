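; Base 2D flipbook monster that wanders around its spawn point, chases the player along X and trades contact damage with them.
; Tick drives an enum state machine that sets direction, walk speed, movement and sprite.
; Chasing starts from facing, distance and line-trace checks, and reverts to walking beyond a leash distance.
; Overlap hurts both sides, sustained contact drains only monster health, and death destroys it after a delay.
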(event `self.ReceiveActorBeginOverlap`
  (params (OtherActor :type "Actor Object Reference"))
  ;[1 1 1] Begin Damage To Player
  (if (`self.ActorHasTag` OtherActor (`self.damageplayer`))
    (bind _aschar_zkx (cast `/Game/demo/blueprint/char_zkx` OtherActor))
    (`self.damage_player` _aschar_zkx)
    (set `self.BeforeOverlapTme` (`GameplayStatics.GetTimeSeconds`))
    (set `self.MonsterHealthValue` (- (`self.MonsterHealthValue`) 0.1))))

(event `self.ReceiveBeginPlay`
  ;[1 1 1] BeginPlay
  (`self.init`))

(event `self.ReceiveTick`
  (params (DeltaSeconds :type "Float (single-precision)"))
  ;[1 1 1] Tick
  (`|ExecutionSequence`
    (:`then_0`
      (`self.ConvertState`))
    (:`then_1`
      (`self.SetMoveDirectionSpeed`)
      (`self.SetisMovingRight`)
      (`self.curtomodespeed`))
    (:`then_2`
      (bind _ismove (`self.IsMove`))
      (if _ismove
        (`self.monster_move`)))
    (:`then_3`
      (bind _isdamage (`self.IsDamage`))
      (if _isdamage
        (`self.ComputeDamage`)))
    (:`then_4`
      (`self.ChangeHealthWidget`))
    (:`then_5`
      (`self.UpdateAnimation`))
    (:`then_6`
      (bind _isdead (`self.IsDead`))
      (if _isdead
        (set `self.state` "NewEnumerator5")
        (set `self.dead` true)
        (`KismetSystemLibrary.Delay` 2.0)
        (`self.HandDead`)))))

(event `UpdateAnimation`
  ;[1 1 1] Handle Animation
  (`self.ChangeSprite`))

(event `self.OnLanded`
  (params (Hit :type "HitResult Structure (by ref)"))
  ;[1 1 1] OnLand Begin Walking
  (`self.Beginwalking`)
  (`self.ChangeOrientToPlayer`))

(fn `BeginLineTrace`
  (returns (toRunning :type Boolean))
  (bind _returnvalue (`GameplayStatics.GetActorOfClass` "/Game/demo/blueprint/char_zkx.char_zkx_C"))
  (bind (_outhit _returnvalue_2) (`KismetSystemLibrary.LineTraceSingle` (+ (`self.K2_GetActorLocation`) (0.0 0.0 30.0)) (+ (`self.K2_GetActorLocation` _returnvalue) (0.0 0.0 30.0)) "TraceTypeQuery1"))
  (if _returnvalue_2
    (if (`self.ActorHasTag` (`.HitActor` (`GameplayStatics.BreakHitResult` _outhit)) (`self.see`))
      (return false)
      (else
        _)))
  (return true))

(fn `Beginwalking`
  (set `self.state` "NewEnumerator6")
  (set `self.BeforeWalkingTime` (`GameplayStatics.GetTimeSeconds`)))

(fn `BeyondWalkingDistance`
  (returns (beyond :type Boolean))
  (return (> (`KismetMathLibrary.Abs` (- (.x (`self.K2_GetActorLocation`)) (.x (`self.birthpoint`)))) (`self.maxwanderdistance`))))

(fn `ChangeHealthWidget`
  (bind _asmonster_health (cast `/Game/demo/blueprint/MonsterHealth` (`WidgetComponent.GetUserWidgetObject` (`self.HealthWidget`))))
  (`ProgressBar.SetPercent` (`/Game/demo/blueprint/MonsterHealth.MonsterFlood` _asmonster_health) (`self.MonsterHealthValue`)))

(fn `ChangeOrientToPlayer`
  (bind _returnvalue (`GameplayStatics.GetActorOfClass` "/Game/demo/blueprint/char_zkx.char_zkx_C"))
  (if (>= (.x (- (`self.K2_GetActorLocation` _returnvalue) (`self.K2_GetActorLocation`))) 0.0)
    (set `self.bisMovingRight` true)
    (else
      (set `self.bisMovingRight` false))))

(fn `ChangeSprite`
  (switch `/Game/demo/blueprint/EnumState` (`self.state`)
    (:`NewEnumerator0`
      (`PaperFlipbookComponent.SetFlipbook` (`self.Sprite`) "/Game/demo/sprites/monster/fire/Standing.Standing"))
    (:`NewEnumerator1`
      (`PaperFlipbookComponent.SetFlipbook` (`self.Sprite`) (select `bool` (`self.bisMovingRight`) :`false` "/Game/demo/sprites/monster/fire/runmoveleft.runmoveleft" :`true` "/Game/demo/sprites/monster/fire/runmoveright.runmoveright" :!type "PaperFlipbook Object Reference")))
    (:`NewEnumerator2`
      (`PaperFlipbookComponent.SetFlipbook` (`self.Sprite`) "/Game/demo/sprites/monster/fire/jumping.jumping"))
    (:`NewEnumerator5`
      (`PaperFlipbookComponent.SetFlipbook` (`self.Sprite`) "/Game/demo/sprites/monster/fire/dead.dead"))
    (:`NewEnumerator6`
      (`PaperFlipbookComponent.SetFlipbook` (`self.Sprite`) (select `bool` (`self.bisMovingRight`) :`false` "/Game/demo/sprites/monster/fire/moveleft.moveleft" :`true` "/Game/demo/sprites/monster/fire/moveright.moveright" :!type "PaperFlipbook Object Reference")))
    (:`NewEnumerator7`
      (`PaperFlipbookComponent.SetFlipbook` (`self.Sprite`) "/Game/demo/sprites/monster/fire/throwing.throwing"))))

(fn `ComputeDamage`
  (`|ExecutionSequence`
    (:`then_0`
      (`self.DamageToPlayer`))
    (:`then_1`
      (`self.DamageByPlayer`)
      (`self.DamagedAndTurn`))))

(fn `ConvertState`
  (switch `/Game/demo/blueprint/EnumState` (`self.state`)
    (:`NewEnumerator0`
      (bind _torunning (`self.IsStandingToRunning`))
      (if _torunning
        (set `self.state` "NewEnumerator1")))
    (:`NewEnumerator1`
      (bind _tostanding (`self.IsRunningToStanding`))
      (if _tostanding
        (set `self.state` "NewEnumerator0")
        (else
          (bind _towaiking (`self.IsRuningToWalking`))
          (if _towaiking
            (`self.Beginwalking`)))))
    (:`NewEnumerator6`
      (bind _torunning_2 (`self.IsWalkingToRunning`))
      (if _torunning_2
        (set `self.state` "NewEnumerator1")))))

(fn `curtomodespeed`
  (set `CharacterMovementComponent.MaxWalkSpeed` (`self.curspeed`) (`self.CharacterMovement`)))

(fn `damage_player`
  (params (player :type "/Game/demo/blueprint/char_zkx Object Reference"))
  (set `/Game/demo/blueprint/char_zkx.HealthCurrent` (- (`/Game/demo/blueprint/char_zkx.HealthCurrent` player) (`self.damage`)) player))

(fn `DamageByPlayer`
  (bind _returnvalue (`GameplayStatics.GetActorOfClass` "/Game/demo/blueprint/char_zkx.char_zkx_C"))
  (if (`self.IsOverlappingActor` _returnvalue)
    (if (> (- (`GameplayStatics.GetTimeSeconds`) (`self.BeforeOverlapTme`)) (`self.overlaptime`))
      (set `self.MonsterHealthValue` (- (`self.MonsterHealthValue`) 0.1))
      (set `self.BeforeOverlapTme` (`GameplayStatics.GetTimeSeconds`)))))

(fn `DamagedAndTurn`
  (if (< (`self.MonsterHealthValue`) (`self.lasttickhealth`))
    (`self.ChangeOrientToPlayer`)))

(fn `DamageToPlayer`)

(fn `HandDead`
  (`self.K2_DestroyActor`))

(fn `init`
  (bind _charactermovement (`self.CharacterMovement`))
  (`self.Beginwalking`)
  (`CharacterMovementComponent.SetMovementMode` _charactermovement "MOVE_Walking" 0)
  (set `CharacterMovementComponent.MaxWalkSpeed` 200.0 _charactermovement)
  (set `self.birthpoint` (`self.K2_GetActorLocation`))
  (set `self.directionvector` (1.0 0.0 0.0)))

(fn `initrevivecount`
  (params (revivecount :type Integer))
  (set `self.maxrevivecount` revivecount))

(fn `IsDamage`
  (returns (isdamage :type Boolean))
  (return (not (`self.dead`))))

(fn `IsDead`
  (returns (isdead :type Boolean))
  (if (<= (`self.MonsterHealthValue`) 0.0)
    (return true)
    (else
      (return false))))

(fn `isLinetrace`
  (returns (result :type Boolean))
  (bind _returnvalue (`self.K2_GetActorLocation`))
  (bind _returnvalue_2 (`GameplayStatics.GetActorOfClass` "/Game/demo/blueprint/char_zkx.char_zkx_C"))
  (bind _returnvalue_3 (`self.K2_GetActorLocation` _returnvalue_2))
  (if (>= (.x (- _returnvalue_3 _returnvalue)) 0.0)
    (set `self.ismonstermoveright` true)
    (else
      (set `self.ismonstermoveright` false)))
  (if (xor (`self.bisMovingRight`) (`self.ismonstermoveright`))
    _
    (elif (> (`KismetMathLibrary.Vector_Distance` _returnvalue_3 _returnvalue) (`self.beginrunningdistance`))
      _
      (else
        (return true))))
  (return false))

(fn `IsMove`
  (returns (ismove :type Boolean))
  (return (not (`self.dead`))))

(fn `IsRuningToWalking`
  (returns (ToWaiking :type Boolean))
  (return (> (`KismetMathLibrary.Abs` (- (.x (`self.K2_GetActorLocation`)) (.x (`self.birthpoint`)))) (`self.maxrundistance`))))

(fn `IsRunningToStanding`
  (returns (toStanding :type Boolean))
  (bind _returnvalue (`GameplayStatics.GetActorOfClass` "/Game/demo/blueprint/char_zkx.char_zkx_C"))
  (if (<= (`KismetMathLibrary.Abs` (.x (- (`self.K2_GetActorLocation` _returnvalue) (`self.K2_GetActorLocation`)))) 5.0)
    (return true)
    (else
      (return false))))

(fn `IsStandingToRunning`
  (returns (toRunning :type Boolean))
  (bind _returnvalue (`GameplayStatics.GetActorOfClass` "/Game/demo/blueprint/char_zkx.char_zkx_C"))
  (if (>= (`KismetMathLibrary.Abs` (.x (- (`self.K2_GetActorLocation` _returnvalue) (`self.K2_GetActorLocation`)))) 20.0)
    (return true)
    (else
      (return false))))

(fn `IsWalkingToRunning`
  (returns (torunning :type Boolean))
  (bind _beyond (`self.BeyondWalkingDistance`))
  (if (not _beyond)
    (bind _result (`self.isLinetrace`))
    (if _result
      (bind _torunning (`self.BeginLineTrace`))
      (return _torunning))))

(fn `monster_move`
  (`self.AddMovementInput` (`self.directionvector`)))

(fn `SetisMovingRight`
  (if (> (.x (`self.directionvector`)) 0.0)
    (set `self.bisMovingRight` true)
    (else
      (set `self.bisMovingRight` false))))

(fn `SetMoveDirectionSpeed`
  (bind _returnvalue (- (.x (`self.K2_GetActorLocation`)) (.x (`self.birthpoint`))))
  (switch `/Game/demo/blueprint/EnumState` (`self.state`)
    (:`NewEnumerator0`
      (set `self.curspeed` 0.0 :!label _label))
    (:`NewEnumerator1`
      (bind _returnvalue_2 (`GameplayStatics.GetActorOfClass` "/Game/demo/blueprint/char_zkx.char_zkx_C"))
      (if (>= (.x (- (`self.K2_GetActorLocation` _returnvalue_2) (`self.K2_GetActorLocation`))) 0.0)
        (set `self.direction` 1.0)
        (else
          (set `self.direction` -1.0)))
      (set `self.directionvector` (`KismetMathLibrary.MakeVector` (`self.direction`)))
      (set `self.curspeed` (`self.runningspeed`)))
    (:`NewEnumerator5`
      (goto _label))
    (:`NewEnumerator6`
      (set `self.curspeed` (`self.walkingspeed`))
      (if (> (`KismetMathLibrary.Abs` _returnvalue) (`self.maxwanderdistance`))
        (if (> _returnvalue 0.0)
          (set `self.direction` -1.0)
          (else
            (set `self.direction` 1.0)))
        (set `self.directionvector` (`KismetMathLibrary.MakeVector` (`self.direction`)))))
    (:`NewEnumerator7`
      (set `self.directionvector` (`self.throwdircection`))
      (set `self.curspeed` (`self.throwspeed`)))))

(fn `SetThrowing`
  (set `self.state` "NewEnumerator7"))

(fn `UserConstructionScript`)