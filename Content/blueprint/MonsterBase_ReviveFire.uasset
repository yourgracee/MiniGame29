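; MonsterBase_ReviveFire is a monster Blueprint that revives a limited number of times when it dies.
; The HandDead event calls Revive, which destroys the actor and, while revives remain, decrements the count and spawns a new instance of the same class at its transform.
; The replacement receives a default controller and the remaining count through Initrevivecount, so the limit carries across each respawn.
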(event `self.HandDead`
  (`self.revive`))

(fn `revive`
  (`self.K2_DestroyActor`)
  (if (> (`self.maxrevivecount`) 0)
    (set `self.maxrevivecount` (- (`self.maxrevivecount`) 1))
    (bind _returnvalue (`|SpawnActorFromClass` "MonsterBase_ReviveFire_C" (`self.GetTransform`) "AlwaysSpawn" "OverrideRootScale" null null))
    (`self.SpawnDefaultController` _returnvalue)
    (`self.initrevivecount` _returnvalue (`self.maxrevivecount`))))

(fn `UserConstructionScript`
  (`parent.UserConstructionScript`))